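; Health component for enemy actors that tracks damage, death and two damage-over-time effects: bullet burn and holy water.
; On BeginPlay it fills health and binds to the owner's any-damage event, clamping health, broadcasting changes, and firing OnDeath once with the damage causer.
; Each effect runs a looping timer that applies damage back through that same path.
; Restarting an effect resets its end timer without stacking ticks.
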(event Custom|HandleDamage
  (params (DamagedActor :type Actor%20Object%20Reference) (Damage :type Float%20%28single-precision%29) (DamageType :type Damage%20Type%20Object%20Reference) (InstigatedBy :type Controller%20Object%20Reference) (DamageCauser :type Actor%20Object%20Reference))
  (if (not (or (Variables|Default|GetbIsDead) (<= Damage 0.0)))
    (bind _output_get (Variables|Default|SetCurrentHealth (Math|Float|Clamp(Float) (- (Variables|Default|GetCurrentHealth) Damage) 0.0 (Variables|Default|GetMaxHealth))))
    (Default|CallOnHealthChanged _output_get (* Damage -1.0))
    (if (<= (Variables|Default|GetCurrentHealth) 0.0)
      (Variables|Default|SetbIsDead true)
      (Default|CallOnDeath DamageCauser (Components|GetOwner)))))

(event Custom|StartBurn
  (bind _self self)
  (Utilities|Time|SetTimerbyFunctionName _self "EndBulletBurn" 10.0001)
  (if (not (Class|KismetSystemLibrary|IsTimerActive _self "BulletBurnTick"))
    (Utilities|Time|SetTimerbyFunctionName _self "BulletBurnTick" 0.5 true)))

(event Custom|EndBulletBurn
  (Utilities|Time|ClearTimerbyFunctionName self "BulletBurnTick"))

(event Custom|BulletBurnTick
  (Game|Damage|ApplyDamage (Components|GetOwner) 2.0 0 0))

(event Custom|StartHolyWater
  (bind _self self)
  (Utilities|Time|SetTimerbyFunctionName _self "EndHolyWater" 5.0001)
  (if (not (Class|KismetSystemLibrary|IsTimerActive _self "HolyWaterTick"))
    (Utilities|Time|SetTimerbyFunctionName _self "HolyWaterTick" 0.2 true)))

(event Custom|EndHolyWater
  (Utilities|Time|ClearTimerbyFunctionName self "HolyWaterTick"))

(event Custom|HolyWaterTick
  (Game|Damage|ApplyDamage (Components|GetOwner) 3.0 0 0))

(event EventBeginPlay
  (Variables|Default|SetCurrentHealth (Variables|Default|GetMaxHealth))
  (EventDispatchers|BindEventtoOnTakeAnyDamage (Components|GetOwner) (delegate Custom|HandleDamage)))

(event EventTick
  (params (DeltaSeconds :type Float%20%28single-precision%29)))