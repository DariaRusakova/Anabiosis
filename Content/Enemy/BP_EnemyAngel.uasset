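; BP_EnemyAngel is an enemy angel that can be set on fire and reports its death to the quest HUD.
; ApplyFireStatus starts burning through the BPCHealth component, refreshing burn time from fire bullets or floor.
; When destroyed while dead, it casts the player HUD to BP_QuestHUD and calls CountAngels.
; The Hit event is empty, and an older tag-checked fire-bullet burn path is left unconnected.
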(event Custom|ApplyFireStatus
  (Default|StartBurn (Variables|Default|GetBPC_Health)))

(event Collision|EventHit
  (params (MyComp :type Primitive%20Component%20Object%20Reference) (Other :type Actor%20Object%20Reference) (OtherComp :type Primitive%20Component%20Object%20Reference) (bSelfMoved :type Boolean) (HitLocation :type Vector :default "0, 0, 0") (HitNormal :type Vector :default "0, 0, 0") (NormalImpulse :type Vector :default "0, 0, 0") (Hit :type Hit%20Result%20Structure%20%28by%20ref%29)))

(event EventDestroyed
  (if (Variables|/Game/Enemy/BPC_Health.BPC_Health_C|GetbIsDead (Variables|Default|GetBPC_Health))
    (bind _asbp_quest_hud (Utilities|Casting|CastToBP_QuestHUD (HUD|GetHUD (Game|GetPlayerController 0))))
    (Default|CountAngels _asbp_quest_hud)))

(fn ConstructionScript
  (|CallParentFunction))