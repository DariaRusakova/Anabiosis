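; Enemy AI pawn that spots the first-person player and takes damage from bullets.
; Pawn sensing sets the HasSeenPlayer blackboard key on sighting, while the older chase-and-attack montage logic sits disconnected.
; Fire and water bullet hits both call StartBurn on the health component.
; Destruction follows either the component's OnDeath or a separate Health variable that AnyDamage reduces to zero.
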(event OnSeePawn(PawnSensing)
  (params (Pawn :type Pawn%20Object%20Reference))
  (Utilities|Casting|CastToBP_FirstPersonCharacter Pawn)
  (AI|Components|Blackboard|SetValueasBool (AI|GetBlackboard (AI|GetAIController self)) (Utilities|Name|MakeLiteralName "HasSeenPlayer") true))

(event OnDeath(BPC_Health)
  (params (Killer :type Actor%20Object%20Reference) (DeadActor :type Actor%20Object%20Reference))
  (Actor|DestroyActor))

(event Custom|FollowPlayer)

(event EventBeginPlay
  ;[0.15 0.15 0.15 0.5] Проверка - урон работает
)

(event Collision|EventActorBeginOverlap
  (params (OtherActor :type Actor%20Object%20Reference)))

(event EventTick
  (params (DeltaSeconds :type Float%20%28single-precision%29)))

(event Game|Damage|EventAnyDamage
  (params (Damage :type Float%20%28single-precision%29) (DamageType :type Damage%20Type%20Object%20Reference) (InstigatedBy :type Controller%20Object%20Reference) (DamageCauser :type Actor%20Object%20Reference))
  ;[0.15 0.15 0.15 0.5] Урон по енемису
  (bind _output_get (Variables|Default|SetHealth (- (Variables|Default|GetHealth) Damage)))
  (if (<= _output_get 0.0)
    (Actor|DestroyActor)))

(event Collision|EventHit
  (params (MyComp :type Primitive%20Component%20Object%20Reference) (Other :type Actor%20Object%20Reference) (OtherComp :type Primitive%20Component%20Object%20Reference) (bSelfMoved :type Boolean) (HitLocation :type Vector :default "0, 0, 0") (HitNormal :type Vector :default "0, 0, 0") (NormalImpulse :type Vector :default "0, 0, 0") (Hit :type Hit%20Result%20Structure%20%28by%20ref%29))
  (Utilities|Casting|CastToBP_BulletFire Other
    (:then
      _)
    (:CastFailed
      (Utilities|Casting|CastToBP_BulletWater Other)))
  (Default|StartBurn (Variables|Default|GetBPC_Health)))

(fn ConstructionScript)