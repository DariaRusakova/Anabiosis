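; HUD Blueprint that runs the angel's quest: offer, kill tracking and a double-jump reward.
; DrawHUD paints everything on the canvas and polls input: near BP_QuestAngel, any key press (prompt says E) opens a Yes/No hit-box dialog.
; CountDemons and CountAngels count only while active and share one completion check requiring both targets, though only demons are displayed, against a hard-coded 20.
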(event Custom|CountDemons
  (if (Variables|Default|GetQuestActive)
    (Variables|Default|SetDemonsKilled (+ (Variables|Default|GetDemonsKilled) 1))
    (if (and (>= (Variables|Default|GetDemonsKilled) (Variables|Default|GetDemonsRequired)) (>= (Variables|Default|GetAngelsKilled) (Variables|Default|GetAngelsRequired)))
      (Variables|Default|SetQuestActive false)
      (Variables|Default|SetQuestComplete true)
      (Variables|/Script/Engine.Character|SetJumpMaxCount (Game|GetPlayerCharacter 0) 2) ; Однократная награда при выполнении обеих целей.
      (Development|PrintString "Задание выполнено. Открыт двойной прыжок!" true true "(R=0.000000,G=0.660000,B=1.000000,A=1.000000)" 4.0))))

(event Custom|CountAngels
  (if (Variables|Default|GetQuestActive)
    (Variables|Default|SetAngelsKilled (+ (Variables|Default|GetAngelsKilled) 1))
    (if (and (>= (Variables|Default|GetDemonsKilled) (Variables|Default|GetDemonsRequired)) (>= (Variables|Default|GetAngelsKilled) (Variables|Default|GetAngelsRequired)))
      (Variables|Default|SetQuestActive false)
      (Variables|Default|SetQuestComplete true)
      (Variables|/Script/Engine.Character|SetJumpMaxCount (Game|GetPlayerCharacter 0) 2) ; Однократная награда при выполнении обеих целей.
      (Development|PrintString "Задание выполнено. Открыт двойной прыжок!" true true "(R=0.000000,G=0.660000,B=1.000000,A=1.000000)" 4.0))))

(event EventDrawHUD
  (params (SizeX :type Integer) (SizeY :type Integer))
  (if (Variables|Default|GetOfferOpen)
    (HUD|DrawRect "(R=0.025,G=0.032,B=0.05,A=0.97)" 24.0 54.0 4.3e+02 186.0)
    (HUD|DrawText "Ангел: победи 20 демонов." "(R=1,G=1,B=1,A=1)" 44.0 7e+01 0 1.3 false)
    (HUD|DrawText "Награда: двойной прыжок" "(R=1,G=1,B=1,A=1)" 44.0 103.0 0 1.3 false)
    (HUD|DrawRect "(R=0.04,G=0.60,B=0.14,A=1)" 44.0 146.0 72.0 72.0)
    (HUD|DrawText "Да" "(R=1,G=1,B=1,A=1)" 56.0 171.0 0 1.3 false)
    (Class|HUD|AddHitBox "(X=44.000000,Y=146.000000)" "(X=72.000000,Y=72.000000)" "Yes" true)
    (HUD|DrawRect "(R=0.7,G=0.05,B=0.05,A=1)" 144.0 146.0 72.0 72.0)
    (HUD|DrawText "Нет" "(R=1,G=1,B=1,A=1)" 156.0 171.0 0 1.3 false)
    (Class|HUD|AddHitBox "(X=144.000000,Y=146.000000)" "(X=72.000000,Y=72.000000)" "No" true)
    (elif (not (Variables|Default|GetQuestComplete))
      (if (Variables|Default|GetQuestActive)
        (HUD|DrawText "Демоны:" "(R=1,G=1,B=1,A=1)" 24.0 32.0 0 1.3 false)
        (HUD|DrawText (Utilities|String|ToString(Integer) (Variables|Default|GetDemonsKilled)) "(R=1,G=1,B=1,A=1)" 115.0 32.0 0 1.3 false)
        (HUD|DrawText "/ 20" "(R=1,G=1,B=1,A=1)" 149.0 32.0 0 1.3 false)
        (else
          (bind _returnvalue (Actor|GetActorOfClass "/Game/Quests/BP_QuestAngel.BP_QuestAngel_C"))
          (if (Utilities|IsValid _returnvalue)
            (if (<= (Transformation|GetDistanceTo _returnvalue (Game|GetPlayerCharacter 0)) 2.4e+02)
              (HUD|DrawText "E — поговорить с ангелом" "(R=1,G=1,B=1,A=1)" 24.0 32.0 0 1.3 false)
              (if (Game|Player|WasInputKeyJustPressed (Game|GetPlayerController 0) "AnyKey")
                (Variables|Default|SetOfferOpen true)
                (Variables|/Script/Engine.PlayerController|SetbShowMouseCursor (Game|GetPlayerController 0) true)
                (Variables|/Script/Engine.PlayerController|SetbEnableClickEvents (Game|GetPlayerController 0) true)
                (Input|SetInputModeGameandUI (Game|GetPlayerController 0) 0 "DoNotLock" true false)))))))))

(event EventHitBoxClick
  (params (BoxName :type Name :default "None"))
  (if (Variables|Default|GetOfferOpen)
    (Variables|Default|SetOfferOpen false)
    (Variables|/Script/Engine.PlayerController|SetbShowMouseCursor (Game|GetPlayerController 0) false)
    (Input|SetInputModeGameOnly (Game|GetPlayerController 0) false)
    (if (Utilities|Name|Equal(Name) BoxName "Yes")
      (Variables|Default|SetQuestActive true))))

(fn ConstructionScript)